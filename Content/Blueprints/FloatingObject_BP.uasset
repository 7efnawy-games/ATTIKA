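; Floating physics object that bobs on water and can be grabbed by the third-person character.
; Tick applies BuoyancyFunction at four corner points, each taking an equal share of the mesh's mass.
; GrabMe traces toward the player pawn, grabs the hit component with a PhysicsHandle and stores the character.
; While grabbed, Tick matches the character's height to the object and holds the object ahead, turned sideways to the character.
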(event `self.ReceiveTick`
  (params (DeltaSeconds :type "Float (single-precision)"))
  (bind _cornerpositions (`self.CornerPositions`))
  (bind _grabbedactor (`self.GrabbedActor`))
  (bind _mesh (`self.Mesh`))
  (bind _returnvalue (`self.K2_GetActorLocation` _grabbedactor))
  (for _array_element _cornerpositions
    (`/Game/Blueprints/passive/WaterBodyFunctions.BuoyancyFunction` _mesh 418.0 (`SceneComponent.K2_GetComponentLocation` _array_element) (/ (`PrimitiveComponent.GetMass` _mesh) (`KismetMathLibrary.Conv_IntToDouble` (`KismetArrayLibrary.Array_Length` _cornerpositions))))
    (if (`self.Grabbed`)
      (`self.K2_SetActorLocation` _grabbedactor (`KismetMathLibrary.MakeVector` (.x _returnvalue) (.y _returnvalue) (.z (`self.K2_GetActorLocation`))) false false)
      (`self.K2_SetActorLocation` (+ _returnvalue (* (`SceneComponent.GetForwardVector` (`Actor.RootComponent` _grabbedactor)) 100.0)))
      (`self.K2_SetActorRotation` (`KismetMathLibrary.MakeRotator` (.roll (`self.K2_GetActorRotation` _grabbedactor)) (.pitch (`self.K2_GetActorRotation` _grabbedactor)) (+ (.yaw (`self.K2_GetActorRotation` _grabbedactor)) 90.0))))))

(fn `GrabMe`
  (bind _returnvalue (`self.K2_GetActorLocation`))
  (bind _outhit (`KismetSystemLibrary.LineTraceSingleForObjects` :`Start` _returnvalue :`End` (`KismetMathLibrary.MakeVector` (.x (`self.K2_GetActorLocation` (`Controller.K2_GetPawn` (`GameplayStatics.GetPlayerController` 0)))) (.y (`self.K2_GetActorLocation` (`Controller.K2_GetPawn` (`GameplayStatics.GetPlayerController` 0)))) (.z _returnvalue)) :`ObjectTypes` (`|MakeArray` (enumliteral `EObjectTypeQuery` "ObjectTypeQuery3")) :`DrawDebugType` "Persistent"))
  (bind (_bblockinghit _binitialoverlap _time _distance _location _impactpoint _normal _impactnormal _physmat _hitactor _hitcomponent _hitbonename _hititem _faceindex _tracestart _traceend) (`GameplayStatics.BreakHitResult` _outhit))
  (`PhysicsHandleComponent.GrabComponentAtLocation` (`self.PhysicsHandle`) _hitcomponent "None" _traceend)
  (set `self.Grabbed` true)
  (bind _asthird_person_character (cast `/Game/ThirdPersonBP/Blueprints/ThirdPersonCharacter` _hitactor))
  (set `self.GrabbedActor` _asthird_person_character))

(fn `UserConstructionScript`
  (set `self.CornerPositions` (`|MakeArray` (`self.CornerPosition1`) (`self.CornerPosition2`) (`self.CornerPosition3`) (`self.CornerPosition4`)))
  (set `self.ObjectTypes` (`|MakeArray` (enumliteral `EObjectTypeQuery` "ObjectTypeQuery4")))
  (set `self.Grabbed` false))