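; Helper functions for the reactive water system that trigger surface disturbances and float physics objects.
; Impact and rain functions find every WaterBody_BP0 actor, copy in location, size and strength parameters, then fire its manual impact or raindrop.
; Buoyancy traces down from a point and, on a hit, pushes the component along the surface normal with mass-scaled force that weakens with hit distance, setting linear and angular damping.
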(fn `BuoyancyFunction`
  (params (PhysicsComponentToFloat :type "PrimitiveComponent Object Reference") (BuoyancyStart :type "Float (double-precision)" :default 400.0) (PointLoction :type "Vector Structure") (Mass :type "Float (double-precision)") (CollisionChannel :type "EObjectTypeQuery Enum" :default "ObjectTypeQuery7"))
  (bind (_returnvalue_x _returnvalue_y _returnvalue_z) (`KismetMathLibrary.BreakVector` (`SceneComponent.K2_GetComponentScale` PhysicsComponentToFloat)))
  (bind (_outhit _returnvalue) (`KismetSystemLibrary.LineTraceSingleForObjects` null PointLoction (- PointLoction (`KismetMathLibrary.MakeVector` 0.0 0.0 (+ (/ (+ _returnvalue_x _returnvalue_y _returnvalue_z) 3.0) BuoyancyStart))) (`|MakeArray` CollisionChannel)))
  (if _returnvalue
    (bind (_bblockinghit _binitialoverlap _time _distance _location _impactpoint _normal _impactnormal) (`GameplayStatics.BreakHitResult` _outhit))
    (`PrimitiveComponent.AddForceAtLocation` PhysicsComponentToFloat (* _impactnormal (`KismetMathLibrary.Lerp` (* Mass 6000.0) 0.0 (/ (`KismetMathLibrary.VSize` (- _location PointLoction)) (* BuoyancyStart 1.0)))) PointLoction "None")
    (`PrimitiveComponent.SetLinearDamping` PhysicsComponentToFloat 1.0)
    (`PrimitiveComponent.SetAngularDamping` PhysicsComponentToFloat 1.0)))

(fn `Impact at Location`
  (params (ImpactLocation :type "Vector Structure") (ImpactSize :type "Float (double-precision)" :default 5.0) (ImpactPower :type "Float (double-precision)" :default 1.0))
  (bind _outactors (`GameplayStatics.GetAllActorsOfClass` null "/Game/_Marvelmaster_infinite_reactive_water_/Blueprints/WaterBody_BP0.WaterBody_BP0_C"))
  (for _array_element _outactors
    (set `/Game/_Marvelmaster_infinite_reactive_water_/Blueprints/WaterBody_BP0.ManualImpactLocation` ImpactLocation _array_element)
    (set `/Game/_Marvelmaster_infinite_reactive_water_/Blueprints/WaterBody_BP0.ManualImpactSize` ImpactSize _array_element)
    (set `/Game/_Marvelmaster_infinite_reactive_water_/Blueprints/WaterBody_BP0.ManualImpactPower` ImpactPower _array_element)
    (`/Game/_Marvelmaster_infinite_reactive_water_/Blueprints/WaterBody_BP0.ManualImpact` _array_element)))

(fn `Rain at Location`
  (params (RainLocation :type "Vector Structure") (RainDropLocation :type "Vector Structure") (RainRadius :type Integer) (RainWaveSize :type "Float (double-precision)" :default 5.0) (RainWaveStrenght :type "Float (double-precision)" :default 1.0))
  (bind _outactors (`GameplayStatics.GetAllActorsOfClass` null "/Game/_Marvelmaster_infinite_reactive_water_/Blueprints/WaterBody_BP0.WaterBody_BP0_C"))
  (for _array_element _outactors
    (set `/Game/_Marvelmaster_infinite_reactive_water_/Blueprints/WaterBody_BP0.RainArea` RainLocation _array_element)
    (set `/Game/_Marvelmaster_infinite_reactive_water_/Blueprints/WaterBody_BP0.RainWaveSize` RainWaveSize _array_element)
    (set `/Game/_Marvelmaster_infinite_reactive_water_/Blueprints/WaterBody_BP0.RainWaveStrenght` RainWaveStrenght _array_element)
    (set `/Game/_Marvelmaster_infinite_reactive_water_/Blueprints/WaterBody_BP0.RainDropLoc` RainDropLocation _array_element)
    (`/Game/_Marvelmaster_infinite_reactive_water_/Blueprints/WaterBody_BP0.FireRaindrop` _array_element)))