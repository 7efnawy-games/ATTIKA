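; FloatingObject_BP is a test-point buoyancy actor that keeps a physics-driven sphere component afloat.
; The construction script gathers four child sphere components into an array of sample points.
; Every tick it calls BuoyancyFunction on the main Sphere at each point's world location, using a fixed buoyancy start value and an equal share of the body's mass.
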(event `self.ReceiveTick`
  (params (DeltaSeconds :type "Float (single-precision)"))
  (bind _sphere (`self.Sphere`))
  (bind _spheres (`self.Spheres`))
  (for _array_element _spheres
    (`/Game/_Marvelmaster_infinite_reactive_water_/Blueprints/passive/WaterBodyFunctions.BuoyancyFunction` _sphere 418.0 (`SceneComponent.K2_GetComponentLocation` _array_element) (/ (`PrimitiveComponent.GetMass` _sphere) (`KismetMathLibrary.Conv_IntToDouble` (`KismetArrayLibrary.Array_Length` _spheres))))))

(fn `UserConstructionScript`
  (set `self.Spheres` (`|MakeArray` (`self.Sphere1`) (`self.Sphere2`) (`self.Sphere3`) (`self.Sphere4`))))